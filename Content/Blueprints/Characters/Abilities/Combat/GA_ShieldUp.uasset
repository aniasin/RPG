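; Gameplay Ability that raises a character's shield while its input is held.
; On activation it commits, flags the CharacterV2 as shield-up, applies GE_ShieldUpBP and plays the shield montage, ending on input release or montage end.
; BPEnnemy avatars also receive a reference to the ability instance.
; On end it clears the flag, applies GE_ShieldUpRemovalBP, then immediately removes both effects by handle.
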(event Ability|EventActivateAbility
  (bind _returnvalue (Ability|CommitAbility))
  (if _returnvalue
    (bind _ascharacter_v2 (Utilities|Casting|CastToCharacterV2 (Ability|GetAvatarActorfromActorInfo)))
    (bind _output_get (Variables|Default|SetCurrentCharacter _ascharacter_v2))
    (Class|CharacterV2|IsShieldUp _output_get true)
    (bind _returnvalue_2 (Ability|ApplyGameplayEffectToOwner "/Game/Blueprints/Characters/GameplayEffects/Combat/GE_ShieldUpBP.GE_ShieldUpBP_C" (Ability|GetAbilityLevel)))
    (Variables|Default|SetGE_ShieldUp _returnvalue_2)
    (|PlayMontageandWaitProxy "None" "/Game/CharactersV2/Characters/Mannequin/Animations/Shield_Montage_HS.Shield_Montage_HS" 1.0 "None" true 1.0
      (:then
        (bind _asbpennemy (Utilities|Casting|CastToBPEnnemy (Variables|Default|GetCurrentCharacter))
          (:then
            (Variables|/Game/Blueprints/Characters/BPEnnemy.BPEnnemy_C|SetShieldUp _asbpennemy self))
          (:CastFailed
            _))
        (Ability|Tasks|WaitInputRelease false
          (:OnRelease
            (Ability|EndAbility))))
      (:OnCompleted
        (Ability|EndAbility :!label _label))
      (:OnBlendOut
        (goto _label))
      (:OnInterrupted
        (goto _label))
      (:OnCancelled
        (goto _label)))
    (else
      (goto _label))))

(event Ability|EventOnEndAbility
  (params (bWasCancelled :type Boolean))
  (Class|CharacterV2|IsShieldUp (Variables|Default|GetCurrentCharacter) false)
  (bind _returnvalue (Ability|ApplyGameplayEffectToOwner "/Game/Blueprints/Characters/GameplayEffects/Combat/GE_ShieldUpRemovalBP.GE_ShieldUpRemovalBP_C" (Ability|GetAbilityLevel)))
  (Variables|Default|SetGE_ShieldUpRemoval _returnvalue)
  (Ability|RemoveGameplayEffectFromOwnerWithHandle (Variables|Default|GetGE_ShieldUp))
  (Ability|RemoveGameplayEffectFromOwnerWithHandle (Variables|Default|GetGE_ShieldUpRemoval)))