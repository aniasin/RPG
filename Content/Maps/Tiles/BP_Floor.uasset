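; BP_Floor is a floor tile actor that can spawn a SizeX by SizeY grid of copies of itself through GenerateTiles.
; Arrow components mark neighbor transforms: each line chains northward from the last spawned tile, and new lines start from the previous line's west arrow.
; The construction script gives each tile a dynamic M_Potion_Inst material with one of four random Row values for visual variation.
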(event Custom|GenerateTiles
  (Variables|Default|SetNewlineTransform (CallFunction|GetTileTransformWest))
  (Variables|Default|SetTileTransform (CallFunction|GetTileTransformNorth))
  (CallFunction|CreateLineNorth)
  (for _index (range 0 (- (Variables|Settings|GetSizeY) 2))
    (CallFunction|CreateNewLine)
    (CallFunction|CreateLineNorth)))

(event Custom|CreateLineNorth
  (for _index (range 0 (- (Variables|Settings|GetSizeX) 2))
    (bind _returnvalue (Game|SpawnActorfromClass "BP_Floor_C" (Variables|Default|GetTileTransform) "Undefined" 0 0))
    (Variables|Default|SetTileTransform (CallFunction|GetTileTransformNorth _returnvalue))))

(event Custom|CreateNewLine
  (bind _returnvalue (Game|SpawnActorfromClass "BP_Floor_C" (Variables|Default|GetNewlineTransform) "Undefined" 0 0))
  (Transformation|SetActorRotation _returnvalue "0,0.000000, 0")
  (Variables|Default|SetTileTransform (CallFunction|GetTileTransformNorth _returnvalue))
  (Variables|Default|SetNewlineTransform (CallFunction|GetTileTransformWest _returnvalue)))

(fn ConstructionScript
  (switch int (Math|Random|RandomInteger 4)
    (:0
      (Variables|Default|SetValue 0.0))
    (:1
      (Variables|Default|SetValue 0.125))
    (:2
      (Variables|Default|SetValue 0.25))
    (:3
      (Variables|Default|SetValue 0.375)))
  (bind _returnvalue (Rendering|Material|CreateDynamicMaterialInstance (Variables|Default|GetFloor) 0 "/Game/Maps/Materials/M_Potion_Inst.M_Potion_Inst" "None" :!class /Script/Engine.PrimitiveComponent))
  (Rendering|Material|SetScalarParameterValue _returnvalue "Row" (Variables|Default|GetValue) :!class /Script/Engine.MaterialInstanceDynamic))

(fn GetTileTransformNorth
  (return (Transformation|GetWorldTransform (Variables|Default|GetArrowNorth))))

(fn GetTileTransformSouth
  (return (Transformation|GetWorldTransform (Variables|Default|GetArrowSouth))))

(fn GetTileTransformWest
  (return (Transformation|GetWorldTransform (Variables|Default|GetArrowWest))))

(fn GetTileTransformEast
  (return (Transformation|GetWorldTransform (Variables|Default|GetArrowEast))))