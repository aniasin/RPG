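; GA_MeleeAttackBP is a Gameplay Ability for a right-hand melee attack by CharacterV2.
; After committing, it plays the character's right-hand montage and waits for a single Data.Hit gameplay event.
; On a hit, it applies a damage Gameplay Effect to the event's target, passing the right weapon's damage through SetByCaller.
; The ability ends when the montage finishes or is interrupted, or when the commit, cast or montage check fails.
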(event Ability|EventActivateAbility
  (bind _returnvalue (Ability|CommitAbility))
  (if _returnvalue
    (bind _ascharacter_v2 (Utilities|Casting|CastToCharacterV2 (Ability|GetAvatarActorfromActorInfo))
      (:then
        (bind _output_get (Variables|Default|SetCurrentCharacter _ascharacter_v2))
        (Utilities|IsValid (Variables|/Script/HS.CharacterV2|GetMontageRightHand _output_get)
          (:Is%20Valid
            (|PlayMontageandWaitProxy "None" (Variables|/Script/HS.CharacterV2|GetMontageRightHand _output_get) 1.0 "None" true 1.0
              (:then
                (bind _payload (Ability|Tasks|WaitGameplayEvent "(TagName=\"Data.Hit\")" 0 true)
                  (:EventReceived
                    (bind _returnvalue_2 (Ability|GameplayEffect|AssignTagSetbyCallerMagnitude (Ability|MakeOutgoingGameplayEffectSpec (Variables|Default|GetDamageeGameplayEffectClass) (Math|Conversions|ToFloat(Integer) (Ability|GetAbilityLevel))) "(TagName=\"Data.Damage\")" (Variables|/Script/HS.Weapon|GetDamage (Variables|/Script/HS.CharacterV2|GetWeaponR (Variables|Default|GetCurrentCharacter)))))
                    (GameplayEffects|ApplyGameplayEffectSpecToTarget _returnvalue_2 (Ability|TargetData|AbilityTargetDatafromActor (.target _payload))))))
              (:OnCompleted
                (Ability|EndAbility :!label _label))
              (:OnBlendOut
                (goto _label))
              (:OnInterrupted
                (goto _label))
              (:OnCancelled
                (goto _label))))
          (:Is%20Not%20Valid
            (goto _label))))
      (:CastFailed
        (goto _label)))
    (else
      (goto _label))))