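; Hero character Blueprint handling combat reactions, death and player UI, with death logic that also covers AI-controlled instances.
; BeginPlay binds delegates: death ragdolls the mesh via multicast/server events, notifying AI and unpossessing on authority.
; Hits apply a GAS stun effect and play the weapon's montage, while a separate HitReact event launches the character.
; It also manages an input-aware interaction prompt, a bow crosshair toggle and the Escape game menu.
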(event Custom|HitReact
  (params (Direction :type Vector) (Force :type Float%20%28single-precision%29))
  (Character|LaunchCharacter (* Direction Force) false false)
  (bind _asmister_hero_anim_bp_hs (Utilities|Casting|CastToMisterHero_AnimBP_HS (Components|SkeletalMesh|GetAnimInstance (Variables|Character|GetMesh))))
  (if (not (Variables|/Game/CharactersV2/Characters/Mannequin/Animations/MisterHero_AnimBP_HS.MisterHero_AnimBP_HS_C|GetIsInCombat? _asmister_hero_anim_bp_hs))
    (Transformation|SetActorRotation (Math|Rotator|FindLookatRotation (Transformation|GetActorForwardVector) Direction))))

(event Custom|Server_Death
  (bind _returnvalue (Pawn|GetController))
  ;[1 1 1] Death
  (Collision|SetCollisionEnabled (Variables|Character|GetMesh) "PhysicsOnly")
  (Physics|SetSimulatePhysics (Variables|Character|GetMesh) true)
  (Networking|SwitchHasAuthority
    (:Authority
      (if (== (Utilities|GetClass _returnvalue) "/Script/HS.Npc_AIController")
        (bind _ashs_aicontroller_bp (Utilities|Casting|CastToHS_AIControllerBP _returnvalue)
          (:then
            (Default|OnDeath _ashs_aicontroller_bp))
          (:CastFailed
            _)))
      (Pawn|UnPossess _returnvalue))))

(event Custom|Multicasst_Death
  (bind _returnvalue (Pawn|GetController))
  ;[1 1 1] Death
  (Collision|SetCollisionEnabled (Variables|Character|GetMesh) "PhysicsOnly")
  (Physics|SetSimulatePhysics (Variables|Character|GetMesh) true)
  (Networking|SwitchHasAuthority
    (:Authority
      (if (== (Utilities|GetClass _returnvalue) "/Script/HS.Npc_AIController")
        (bind _ashs_aicontroller_bp (Utilities|Casting|CastToHS_AIControllerBP _returnvalue)
          (:then
            (Default|OnDeath _ashs_aicontroller_bp))
          (:CastFailed
            _)))
      (Pawn|UnPossess _returnvalue))))

(event EventTick
  (params (DeltaSeconds :type Float%20%28single-precision%29))
  ;[1 1 1] TICK
)

(event EventBeginPlay
  ;[0.5724 1 0.6015] BeginPlay
  (Variables|Default|SetHomeLocation (Transformation|GetActorLocation))
  (Utilities|InnitializeInteractionWidget)
  (Variables|Default|SetMontagePickUp "/Game/CharactersV2/Characters/Mannequin/Animations/PickUp_noWeaponAnim_HS_Montage.PickUp_noWeaponAnim_HS_Montage")
  (|OnDeath_DELEGATE)
  (|HitReact_DELEGATE))

(event EventToggleWidget
  (params (bVisibility :type Boolean))
  ;[1 1 1] Interaction Widget
  (Utilities|ToggleInteraction bVisibility))

(event Input|ActionEvents|InputActionEscape
  (params (Key :type Key%20Structure :default "None"))
  ;[1 1 1] LoadGameMenu
  (:Pressed
    (bind _ashsgame_instance (Utilities|Casting|CastToHSGameInstance (Game|GetGameInstance)))
    (Class|HSGameInstance|LoadGameMenu _ashsgame_instance)))

(event Input|ActionEvents|InputActionSwitchCombat
  (params (Key :type Key%20Structure :default "None"))
  ;[1 1 1] CrosHair
  (:Pressed
    (if (== (Utilities|GetClass (Variables|Default|GetWeaponL)) "/Game/Items/BP_Bow.BP_Bow_C")
      (Utilities|FlowControl|FlipFlop
        (:A
          (bind _returnvalue (UserInterface|CreateWidget "/Game/UI/Characters/W_CrossHair.W_CrossHair_C" (Game|GetPlayerController 0)))
          (bind _output_get (Variables|Default|SetCrossHairRef _returnvalue))
          (UserInterface|Viewport|AddtoViewport _output_get 0))
        (:B
          (Widget|RemovefromParent (Variables|Default|GetCrossHairRef)))))))

(fn ConstructionScript)

(event Custom|OnCharacterDied_Event
  (params (Character :type HS%20Character%20Base%20Object%20Reference))
  (if (Ability|HasAuthority)
    (CallFunction|MulticasstDeath)
    (else
      (CallFunction|ServerDeath))))

(event Custom|ShowHitReact_Event
  (params (Direction :type EGDHitReactDirection%20Enum :default "None"))
  (bind _weaponr (Variables|Default|GetWeaponR))
  (bind _weaponl (Variables|Default|GetWeaponL))
  (GameplayEffects|ApplyGameplayEffectToSelf :self (Ability|GetAbilitySystemComponent self) :GameplayEffectClass "/Game/Blueprints/Characters/GameplayEffects/GE_Stun.GE_Stun_C" :Level 1.0)
  (if (Utilities|IsValid _weaponr)
    (Variables|Default|SetGetHitMontage (Variables|/Script/HS.Weapon|GetMontageHit _weaponr))
    (elif (Utilities|IsValid _weaponl)
      (Variables|Default|SetGetHitMontage (Variables|/Script/HS.Weapon|GetMontageHit _weaponl))))
  (Animation|Montage|PlayMontage (Variables|Character|GetMesh) (Variables|Default|GetGetHitMontage)
    (:then
      (return))))