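; Enemy character Blueprint that exposes combat actions for AI through the Gameplay Ability System.
; On BeginPlay it clears its interaction widget and puts its HSCharacterMovementComponent into aim-down-sights.
; AI events activate abilities by class for melee attack, combat switch and shield up.
; Combat switch and shield are FlipFlop toggles that alternate between activating the ability and ending a referenced ability, so they track call order rather than actual ability state.
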(event EventBeginPlay
  (|CallParentFunction)
  (Variables|Default|SetInteractionWidget 0)
  (bind _ashscharacter_movement_component (Utilities|Casting|CastToHSCharacterMovementComponent (Variables|Character|GetCharacterMovement)))
  (Class|HSCharacterMovementComponent|StartAimDownSights _ashscharacter_movement_component))

(event Collision|EventActorBeginOverlap
  (params (OtherActor :type Actor%20Object%20Reference))
  (|CallParentFunction OtherActor))

(event EventTick
  (params (DeltaSeconds :type Float%20%28single-precision%29))
  (|CallParentFunction DeltaSeconds))

(event EventAISwitchCombat
  ;[1 1 1] AISwitchCombat
  (Utilities|FlowControl|FlipFlop
    (:A
      (Abilities|TryActivateAbilitybyClass (Ability|GetAbilitySystemComponent self) "/Game/Blueprints/Characters/Abilities/Combat/GA_SwitchCombatBP.GA_SwitchCombatBP_C" true))
    (:B
      (Ability|EndAbility (Variables|Default|GetSwitchCombatOff)))))

(event EventAIPerformMeleeAttack
  ;[1 1 1] MeleeAttack
  (Abilities|TryActivateAbilitybyClass (Ability|GetAbilitySystemComponent self) "/Game/Blueprints/Characters/Abilities/Combat/GA_MeleeAttackBP.GA_MeleeAttackBP_C" true))

(event EventAIPerformShieldUp
  ;[1 1 1] ShieldUp
  (Utilities|FlowControl|FlipFlop
    (:A
      (Abilities|TryActivateAbilitybyClass (Ability|GetAbilitySystemComponent self) "/Game/Blueprints/Characters/Abilities/Combat/GA_ShieldUp.GA_ShieldUp_C" true))
    (:B
      (Ability|EndAbility (Variables|Default|GetShieldUp)))))

(fn ConstructionScript
  (|CallParentFunction))