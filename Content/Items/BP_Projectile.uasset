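; BP_Projectile is a projectile actor that reports hits to its owning character through the Gameplay Ability System.
; On the authority, a sphere overlap sends a Data.Hit gameplay event to the owner with the target as payload, then destroys the projectile.
; Overlapping the owner destroys it without an event, while BP_Shield only prints a debug message.
; It also destroys itself on a blocking hit or after a fixed lifespan.
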(event OnComponentBeginOverlap(Sphere)
  (params (OverlappedComponent :type Primitive%20Component%20Object%20Reference) (OtherActor :type Actor%20Object%20Reference) (OtherComp :type Primitive%20Component%20Object%20Reference) (OtherBodyIndex :type Integer) (bFromSweep :type Boolean) (SweepResult :type Hit%20Result%20Structure%20%28by%20ref%29))
  (Networking|SwitchHasAuthority
    (:Authority
      (Variables|Default|SetCurrentTarget OtherActor)
      (bind _ascharacter_v2 (Utilities|Casting|CastToCharacterV2 (Variables|Default|GetOwnerActor)))
      (Variables|Default|SetCurrentOwner _ascharacter_v2)
      (if (== (Utilities|GetClass (Variables|Default|GetCurrentTarget)) "/Game/Items/BP_Shield.BP_Shield_C")
        (Development|PrintString "SHIELD!")
        (elif (!= (Variables|Default|GetCurrentOwner) (Variables|Default|GetCurrentTarget))
          (Ability|SendGameplayEventtoActor (Variables|Default|GetCurrentOwner) "(TagName=\"Data.Hit\")" (Utilities|Struct|MakeGameplayEventData "" 0 (Variables|Default|GetCurrentTarget) 0 0 "()" "(GameplayTags=)" "(GameplayTags=)" 0.0 "()"))
          (Development|PrintString "Hit!")
          (Actor|DestroyActor)
          (else
            (Actor|DestroyActor)))))))

(event EventBeginPlay
  (Actor|SetLifeSpan 1e+01))

(event Collision|EventHit
  (params (MyComp :type Primitive%20Component%20Object%20Reference) (Other :type Actor%20Object%20Reference) (OtherComp :type Primitive%20Component%20Object%20Reference) (bSelfMoved :type Boolean) (HitLocation :type Vector :default "0, 0, 0") (HitNormal :type Vector :default "0, 0, 0") (NormalImpulse :type Vector :default "0, 0, 0") (Hit :type Hit%20Result%20Structure%20%28by%20ref%29))
  (Actor|DestroyActor)
  (Development|PrintString (Utilities|GetDisplayName Other)))

(fn ConstructionScript)