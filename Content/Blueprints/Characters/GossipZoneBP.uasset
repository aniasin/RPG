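; GossipZoneBP is a world zone that feeds gossip dialogue to BPEnnemy characters that overlap it.
; It caches its location as Site at BeginPlay.
; On overlap, it adds each Gossips entry to the character's Dialogue array as a timestamped struct with priority, memory duration and site info.
; For civilians in danger zones it only prints a fleeing message per entry, with no flee behavior.
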(event EventBeginPlay
  (Variables|Dialogues|SetSite (Transformation|GetActorLocation)))

(event EventOnOverlapDialogueBegin
  (params (Comp :type Primitive%20Component%20Object%20Reference) (OtherActor :type Actor%20Object%20Reference) (OtherComp :type Primitive%20Component%20Object%20Reference) (OtherBodyIndex :type Integer) (bFromSweep :type Boolean) (HitResult :type Hit%20Result%20Structure%20%28by%20ref%29))
  (if (== (Utilities|GetClass OtherActor) "/Game/Blueprints/Characters/BPEnnemy.BPEnnemy_C")
    (bind _asbpennemy (Utilities|Casting|CastToBPEnnemy OtherActor))
    (bind _output_get (Variables|Default|SetOverlapingActorRef _asbpennemy))
    (for _array_element (Variables|Dialogues|GetGossips)
      (Utilities|Array|AddUnique (Variables|/Script/HS.DialogueComponent|GetDialogArray (Variables|/Game/Blueprints/Characters/BPEnnemy.BPEnnemy_C|GetDialogue _output_get)) (Utilities|Struct|MakeDialogues_Struct (Variables|Dialogues|GetPriority) (Utilities|Time|GetTimeSeconds) (Variables|Dialogues|GetInfoDuration) (Utilities|String|ToString(Text) _array_element) (Variables|Dialogues|GetSite) (Variables|Dialogues|GetSiteName) (Variables|Dialogues|GetPointAt)))
      (if (and (Variables|/Script/HS.CharacterV2|GetbIsCivilian (Variables|Default|GetOverlapingActorRef)) (Variables|Dialogues|GetIsDanger))
        (Development|PrintString (Utilities|String|Append (Utilities|GetDisplayName (Variables|Default|GetOverlapingActorRef)) " IS FLEEING!") true false "(R=1.000000,G=0.076571,B=0.000000,A=1.000000)")))))

(fn ConstructionScript)