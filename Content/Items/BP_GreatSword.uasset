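; BP_GreatSword is a melee weapon that detects hits through its capsule's overlap events, processed only on the server.
; Striking a BP_Shield prints a debug message and plays a dizzy montage on the wielder's mesh.
; Striking a BPHero or BPEnnemy other than the wielder sends a Data.Hit gameplay event to the wielder, with the victim as payload target.
; Targets are matched by exact class, so subclasses do not register.
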(event OnComponentBeginOverlap(CapsuleComponent)
  (params (OverlappedComponent :type Primitive%20Component%20Object%20Reference) (OtherActor :type Actor%20Object%20Reference) (OtherComp :type Primitive%20Component%20Object%20Reference) (OtherBodyIndex :type Integer) (bFromSweep :type Boolean) (SweepResult :type Hit%20Result%20Structure%20%28by%20ref%29))
  (Networking|SwitchHasAuthority
    (:Authority
      (Variables|Default|SetCurrentTarget OtherActor)
      (bind _ascharacter_v2 (Utilities|Casting|CastToCharacterV2 (Variables|Default|GetOwnerActor)))
      (Variables|Default|SetCurrentOwner _ascharacter_v2)
      (if (== (Utilities|GetClass (Variables|Default|GetCurrentTarget)) "/Game/Items/BP_Shield.BP_Shield_C")
        (Development|PrintString "SHIELD!")
        (Animation|Montage|PlayMontage (Variables|/Script/Engine.Character|GetMesh (Variables|Default|GetCurrentOwner)) "/Game/CharactersV2/Characters/Mannequin/Animations/Dizzy_SwordShieldAnim_HS_Montage.Dizzy_SwordShieldAnim_HS_Montage")
        (elif (and (!= (Variables|Default|GetCurrentOwner) (Variables|Default|GetCurrentTarget)) (or (== (Utilities|GetClass (Variables|Default|GetCurrentTarget)) "/Game/Blueprints/Characters/BPHero.BPHero_C") (== (Utilities|GetClass (Variables|Default|GetCurrentTarget)) "/Game/Blueprints/Characters/BPEnnemy.BPEnnemy_C")))
          (Ability|SendGameplayEventtoActor (Variables|Default|GetCurrentOwner) "(TagName=\"Data.Hit\")" (Utilities|Struct|MakeGameplayEventData "" 0 (Variables|Default|GetCurrentTarget) 0 0 "()" "(GameplayTags=)" "(GameplayTags=)" 0.0 "()")))))))

(event EventBeginPlay)

(event Collision|EventActorBeginOverlap
  (params (OtherActor :type Actor%20Object%20Reference)))

(event EventTick
  (params (DeltaSeconds :type Float%20%28single-precision%29)))

(fn ConstructionScript
  (|CallParentFunction))