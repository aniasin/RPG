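; BP_Weapon_Master is a weapon item actor that shows its name as floating text when the hero is nearby.
; BeginPlay writes WeaponName into the TextRender component.
; Sphere overlaps with exactly the BPHero class toggle IsFocused and the text's visibility.
; While focused, Tick turns the text toward the player's view by negating the player controller's pitch and offsetting its yaw by 180 degrees.
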(event OnComponentBeginOverlap(Sphere)
  (params (OverlappedComponent :type Primitive%20Component%20Object%20Reference) (OtherActor :type Actor%20Object%20Reference) (OtherComp :type Primitive%20Component%20Object%20Reference) (OtherBodyIndex :type Integer) (bFromSweep :type Boolean) (SweepResult :type Hit%20Result%20Structure%20%28by%20ref%29))
  (if (== (Utilities|GetClass OtherActor) "/Game/Blueprints/Characters/BPHero.BPHero_C")
    (Variables|Default|SetIsFocused true)
    (Rendering|SetVisibility (Variables|Default|GetTextRender) true false)))

(event OnComponentEndOverlap(Sphere)
  (params (OverlappedComponent :type Primitive%20Component%20Object%20Reference) (OtherActor :type Actor%20Object%20Reference) (OtherComp :type Primitive%20Component%20Object%20Reference) (OtherBodyIndex :type Integer))
  (if (== (Utilities|GetClass OtherActor) "/Game/Blueprints/Characters/BPHero.BPHero_C")
    (Variables|Default|SetIsFocused false)
    (Rendering|SetVisibility (Variables|Default|GetTextRender) false false)))

(event EventBeginPlay
  (Rendering|Components|TextRender|SetText (Variables|Default|GetTextRender) (Variables|Default|GetWeaponName)))

(event Collision|EventActorBeginOverlap
  (params (OtherActor :type Actor%20Object%20Reference)))

(event EventTick
  (params (DeltaSeconds :type Float%20%28single-precision%29))
  (bind _returnvalue (Game|GetPlayerController 0))
  (bind _returnvalue_2 (Transformation|GetActorRotation _returnvalue))
  (bind (_roll _pitch _yaw) (Math|Rotator|BreakRotator _returnvalue_2))
  (if (Variables|Default|GetIsFocused)
    (Transformation|SetWorldRotation (Variables|Default|GetTextRender) (Math|Rotator|MakeRotator (- _roll 0.0) (* _pitch -1.0) (- _yaw 1.8e+02)) false false)))

(fn ConstructionScript)