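; BP_Potion is a potion item actor whose mesh appearance reflects whether it is empty and the sign of its amount.
; The construction script picks a material row for empty, positive amount, or zero-or-negative amount.
; It creates a dynamic material instance on the static mesh and passes that row and the Column variable as scalar parameters.
; The event graph holds no active logic.
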(event EventBeginPlay)

(event Collision|EventActorBeginOverlap
  (params (OtherActor :type Actor%20Object%20Reference)))

(event EventTick
  (params (DeltaSeconds :type Float%20%28single-precision%29)))

(fn ConstructionScript
  (if (Variables|Default|GetbIsEmpty)
    (Variables|Default|SetRow 0.125)
    (elif (> (Variables|Default|GetAmount) 0.0)
      (Variables|Default|SetRow 0.0)
      (else
        (Variables|Default|SetRow 0.5))))
  (bind _returnvalue (Rendering|Material|CreateDynamicMaterialInstance (Variables|Default|GetStaticMesh) 0 0 "None" :!class /Script/Engine.PrimitiveComponent))
  (Rendering|Material|SetScalarParameterValue _returnvalue "Row" (Variables|Default|GetRow) :!class /Script/Engine.MaterialInstanceDynamic)
  (Rendering|Material|SetScalarParameterValue _returnvalue "Column" (Variables|Default|GetColumn) :!class /Script/Engine.MaterialInstanceDynamic))