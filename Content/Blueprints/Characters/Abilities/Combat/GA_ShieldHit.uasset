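; GA_ShieldHit is a gameplay ability that plays the sword-and-shield defend-hit montage on a CharacterV2 avatar.
; On activation it commits, caches the character and ends when the montage finishes, blends out, is interrupted or cancelled, or when commit or cast fails.
; Disconnected leftover nodes for a shield-up effect and hit-event damage from the left-hand weapon never run.
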(event Ability|EventActivateAbility
  (bind _returnvalue (Ability|CommitAbility))
  (if _returnvalue
    (bind _ascharacter_v2 (Utilities|Casting|CastToCharacterV2 (Ability|GetAvatarActorfromActorInfo))
      (:then
        (Variables|Default|SetCurrentCharacter _ascharacter_v2)
        (|PlayMontageandWaitProxy "None" "/Game/CharactersV2/Characters/Mannequin/Animations/DefendHit_SwordShieldAnim_HS_Montage.DefendHit_SwordShieldAnim_HS_Montage" 1.0 "None" true 1.0
          (:OnCompleted
            _)
          (:OnBlendOut
            _)
          (:OnInterrupted
            _)
          (:OnCancelled
            _)))
      (:CastFailed
        _)))
  (Ability|EndAbility))

(event Ability|EventOnEndAbility
  (params (bWasCancelled :type Boolean)))