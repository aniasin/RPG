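; Gameplay ability that toggles the HS character into a combat stance with a drawn right-hand weapon and aim-down-sights movement.
; On activation it applies the switch-combat effect, attaches the weapon, starts aiming on the movement component and waits for another input press to end.
; On end it applies a removal effect, immediately removes both effects by handle, detaches the weapon and stops aiming down sights.
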(event Ability|EventActivateAbility
  (bind _ashscharacter_base (Utilities|Casting|CastToHSCharacterBase (Ability|GetAvatarActorfromActorInfo)))
  (Variables|Default|SetCurrentPlayer _ashscharacter_base)
  (bind _returnvalue (Ability|ApplyGameplayEffectToOwner "/Game/Blueprints/Characters/GameplayEffects/Combat/GE_SwitchCombatBP.GE_SwitchCombatBP_C" (Ability|GetAbilityLevel)))
  (Variables|Default|SetGE_SwitchCombat _returnvalue)
  (Class|HSCharacterBase|AttachWeaponR (Variables|Default|GetCurrentPlayer))
  (bind _ashscharacter_movement_component (Utilities|Casting|CastToHSCharacterMovementComponent (.MovementComponent (Utilities|Struct|BreakGameplayAbilityActorInfo (Ability|GetActorInfo)))))
  (Class|HSCharacterMovementComponent|StartAimDownSights _ashscharacter_movement_component)
  (Ability|Tasks|WaitInputPress false
    (:OnPress
      (Ability|EndAbility))))

(event Ability|EventOnEndAbility
  (params (bWasCancelled :type Boolean))
  (bind _returnvalue (Ability|ApplyGameplayEffectToOwner "/Game/Blueprints/Characters/GameplayEffects/Combat/GE_SwitchCombatRemovalBP.GE_SwitchCombatRemovalBP_C" (Ability|GetAbilityLevel)))
  (Variables|Default|SetGE_SwitchCombatRemoval _returnvalue)
  (Ability|RemoveGameplayEffectFromOwnerWithHandle (Variables|Default|GetGE_SwitchCombat))
  (Ability|RemoveGameplayEffectFromOwnerWithHandle (Variables|Default|GetGE_SwitchCombatRemoval))
  (Class|HSCharacterBase|DetachWeaponR (Variables|Default|GetCurrentPlayer))
  (bind _ashscharacter_movement_component (Utilities|Casting|CastToHSCharacterMovementComponent (.MovementComponent (Utilities|Struct|BreakGameplayAbilityActorInfo (Ability|GetActorInfo)))))
  (Class|HSCharacterMovementComponent|StopAimDownSights _ashscharacter_movement_component))